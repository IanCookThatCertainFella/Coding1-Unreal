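; BP_EnemySpawnManager starts a new enemy wave and spawns a key once no enemies remain.
; NewEnemyWaveCheck looks for BPEnemy actors and, when none are found, calls SpawnNewEnemies and spawns a BPKey at the passed transform.
; SpawnNewEnemies waits on a short delay, then tells every BP_Enemy_Spawner in the level to spawn an enemy.
; BeginPlay also queries the spawners but leaves the result unused.
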(event Custom|NewEnemyWaveCheck
  (params (Transform :type Transform))
  (bind _outactors (Actor|GetAllActorsOfClass "/Game/Blueprints/BPEnemy.BPEnemy_C"))
  (if (not (> (Utilities|Array|Length _outactors) 0))
    (CallFunction|SpawnNewEnemies)
    (Game|SpawnActorfromClass "/Game/Blueprints/BPKey.BPKey_C" Transform "Undefined" "MultiplyWithRoot" 0 0)))

(event Custom|SpawnNewEnemies
  (Utilities|FlowControl|Delay 4.0)
  (bind _outactors (Actor|GetAllActorsOfClass "/Game/Blueprints/BP_Enemy_Spawner.BP_Enemy_Spawner_C"))
  (for (_array_element _array_index) _outactors
    (Default|SpawnNewEnemy _array_element)))

(event EventBeginPlay
  (Actor|GetAllActorsOfClass "/Game/Blueprints/BP_Enemy_Spawner.BP_Enemy_Spawner_C"))

(fn ConstructionScript)