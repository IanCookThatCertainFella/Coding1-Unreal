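; A platform that falls after the third-person character steps into its trigger box, then returns to its start to be used again.
; On overlap it locks itself, waits a fall delay, then enables physics on the mesh for a set duration.
; A timeline then lerps it from the fallen transform back to the saved start transform and rearms it.
; Material swaps show the ready, active, falling and resetting states.
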(event OnComponentBeginOverlap(BoxTrigger)
  (params (OverlappedComponent :type Primitive%20Component%20Object%20Reference) (OtherActor :type Actor%20Object%20Reference) (OtherComp :type Primitive%20Component%20Object%20Reference) (OtherBodyIndex :type Integer) (bFromSweep :type Boolean) (SweepResult :type Hit%20Result%20Structure%20%28by%20ref%29))
  (if (Variables|Default|GetisReady)
    (Utilities|Casting|CastToBP_ThirdPersonCharacter OtherActor)
    (CallFunction|Activate)))

(event Custom|Activate
  (Variables|Default|SetisReady false)
  (Rendering|Material|SetMaterial (Variables|Default|GetPlatform) 0 "/Game/Materials/Falling_Platform/MI_Active_Platform.MI_Active_Platform")
  (Utilities|FlowControl|Delay (Variables|PlatformSettings|GetFall%20Delay%20Duration))
  (CallFunction|Falling))

(event Custom|Falling
  (Rendering|Material|SetMaterial (Variables|Default|GetPlatform) 0 "/Game/Materials/Falling_Platform/MI_Falling_Platform.MI_Falling_Platform")
  (Physics|SetSimulatePhysics (Variables|Default|GetPlatform) true)
  (Utilities|FlowControl|Delay (Variables|Default|GetFall%20Duration))
  (CallFunction|ResetPlatform))

(event Custom|ResetPlatform
  (Rendering|Material|SetMaterial (Variables|Default|GetPlatform) 0 "/Game/Materials/Falling_Platform/MI_Resetting_Platform.MI_Resetting_Platform")
  (Physics|SetSimulatePhysics (Variables|Default|GetPlatform) false)
  (Variables|Default|SetFallen%20Transform (Transformation|GetWorldTransform (Variables|Default|GetPlatform)))
  (bind _newtrack_0 (Timeline|GoBackToStartTransform PlayFromStart)
    (:Update
      (Transformation|SetWorldTransform (Variables|Default|GetPlatform) (Math|Transform|Lerp(Transform) (Variables|Default|GetFallen%20Transform) (Variables|Default|GetStarting%20Transform) _newtrack_0) false false))
    (:Finished
      (Variables|Default|SetisReady true)
      (Rendering|Material|SetMaterial (Variables|Default|GetPlatform) 0 "/Game/Materials/Falling_Platform/MI_Ready_Platform.MI_Ready_Platform"))))

(event EventBeginPlay
  (Variables|Default|SetStarting%20Transform (Transformation|GetWorldTransform (Variables|Default|GetPlatform)))
  (Variables|Default|SetisReady true))

(event Collision|EventActorBeginOverlap
  (params (OtherActor :type Actor%20Object%20Reference)))

(event EventTick
  (params (DeltaSeconds :type Float%20%28single-precision%29)))

(fn ConstructionScript)