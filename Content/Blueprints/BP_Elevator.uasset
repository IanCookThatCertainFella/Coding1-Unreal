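; Elevator actor whose platform travels between a Start and an End point when the third-person character steps into a trigger.
; Bottom and Top overlap volumes call Movement only when the platform is at their end and not already moving.
; Movement plays an up or down timeline that lerps the platform's transform between the two points.
; On finish it flips the position flag and waits briefly before allowing another trip.
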(event OnComponentBeginOverlap(Bottom)
  (params (OverlappedComponent :type Primitive%20Component%20Object%20Reference) (OtherActor :type Actor%20Object%20Reference) (OtherComp :type Primitive%20Component%20Object%20Reference) (OtherBodyIndex :type Integer) (bFromSweep :type Boolean) (SweepResult :type Hit%20Result%20Structure%20%28by%20ref%29))
  (Utilities|Casting|CastToBP_ThirdPersonCharacter OtherActor)
  (Development|PrintString "Hello")
  (if (Variables|Default|GetAt%20Bottom)
    (if (not (Variables|Default|GetIsMoving))
      (CallFunction|Movement))))

(event OnComponentBeginOverlap(Top)
  (params (OverlappedComponent :type Primitive%20Component%20Object%20Reference) (OtherActor :type Actor%20Object%20Reference) (OtherComp :type Primitive%20Component%20Object%20Reference) (OtherBodyIndex :type Integer) (bFromSweep :type Boolean) (SweepResult :type Hit%20Result%20Structure%20%28by%20ref%29))
  (Utilities|Casting|CastToBP_ThirdPersonCharacter OtherActor)
  (if (not (Variables|Default|GetAt%20Bottom))
    (if (not (Variables|Default|GetIsMoving))
      (CallFunction|Movement))))

(event Custom|Movement
  (if (Variables|Default|GetAt%20Bottom)
    (Variables|Default|SetIsMoving true)
    (bind _move_up (Timeline|Timeline PlayFromStart)
      (:Update
        (Transformation|SetWorldLocationAndRotation (Variables|Default|GetPlatform) (.location (Math|Transform|Lerp(Transform) (Transformation|GetWorldTransform (Variables|Default|GetStart)) (Transformation|GetWorldTransform (Variables|Default|GetEnd)) _move_up)) (.rotation (Math|Transform|Lerp(Transform) (Transformation|GetWorldTransform (Variables|Default|GetStart)) (Transformation|GetWorldTransform (Variables|Default|GetEnd)) _move_up)) false false))
      (:Finished
        (Variables|Default|SetAt%20Bottom false)
        (Utilities|FlowControl|Delay 1.0)
        (Variables|Default|SetIsMoving false)))
    (else
      (Variables|Default|SetIsMoving true)
      (bind _move_down (Timeline|Timeline_0 PlayFromStart)
        (:Update
          (Transformation|SetWorldLocationAndRotation (Variables|Default|GetPlatform) (.location (Math|Transform|Lerp(Transform) (Transformation|GetWorldTransform (Variables|Default|GetStart)) (Transformation|GetWorldTransform (Variables|Default|GetEnd)) _move_down)) (.rotation (Math|Transform|Lerp(Transform) (Transformation|GetWorldTransform (Variables|Default|GetStart)) (Transformation|GetWorldTransform (Variables|Default|GetEnd)) _move_down)) false false))
        (:Finished
          (Variables|Default|SetAt%20Bottom true)
          (Utilities|FlowControl|Delay 1.0)
          (Variables|Default|SetIsMoving false))))))

(event EventBeginPlay
  (Variables|Default|SetAt%20Bottom true)
  (Variables|Default|SetTest false)
  (Variables|Default|SetIsMoving false)
  (if (Variables|Default|GetIsMoving)
    _))

(event Collision|EventActorBeginOverlap
  (params (OtherActor :type Actor%20Object%20Reference)))

(event EventTick
  (params (DeltaSeconds :type Float%20%28single-precision%29)))

(fn ConstructionScript)