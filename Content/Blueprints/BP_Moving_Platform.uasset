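; BP_Moving_Platform is a platform actor that travels between a Start and an End transform, starting automatically at BeginPlay.
; A Timeline track drives a transform lerp, setting the platform's world location and rotation on each update.
; The Timeline's Moving and Stopped event tracks swap the platform's material between active and ready looks to signal its state.
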(event EventBeginPlay
  (bind _newtrack_0 (Timeline|Timeline Play)
    (:Update
      (Transformation|SetWorldLocationAndRotation (Variables|Default|GetPlatform) (.location (Math|Transform|Lerp(Transform) (Transformation|GetWorldTransform (Variables|Default|GetStart)) (Transformation|GetWorldTransform (Variables|Default|GetEnd)) _newtrack_0)) (.rotation (Math|Transform|Lerp(Transform) (Transformation|GetWorldTransform (Variables|Default|GetStart)) (Transformation|GetWorldTransform (Variables|Default|GetEnd)) _newtrack_0)) false false))
    (:Moving
      (Rendering|Material|SetMaterial (Variables|Default|GetPlatform) 0 "/Game/Materials/Falling_Platform/MI_Active_Platform.MI_Active_Platform"))
    (:Stopped
      (Rendering|Material|SetMaterial (Variables|Default|GetPlatform) 0 "/Game/Materials/Falling_Platform/MI_Ready_Platform.MI_Ready_Platform"))))

(event Collision|EventActorBeginOverlap
  (params (OtherActor :type Actor%20Object%20Reference)))

(event EventTick
  (params (DeltaSeconds :type Float%20%28single-precision%29)))

(fn ConstructionScript)